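; Inventory component that holds item stacks in a Content slot array, sized to InventorySize on BeginPlay.
; AddItemToInventory places items one at a time, seeking a non-full matching stack, otherwise starting one in an empty slot, and returns success and the leftover quantity.
; Stack limits come from the ItemData table; stack additions always target index 0, not the found slot.
; RemoveFromInventory is an empty stub, and a debug function prints slot contents.
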(event EventBeginPlay
  (Utilities|Array|Resize (Variables|Default|GetContent) (Variables|Default|GetInventorySize)))

(fn AddItemtoInventory
  (params (ItemID :type Name) (Quantity :type Integer))
  (LocalVariables|SetLocal_QuantityRemaining Quantity)
  (while (and (> (LocalVariables|GetLocal_QuantityRemaining) 0) (not (LocalVariables|GetLocal_HasFailed)))
    (bind _foundslot (CallFunction|FindSlot ItemID))
    (if _foundslot
      (CallFunction|AddtoStack 0 1)
      (Math|Integer|DecrementInt (LocalVariables|GetLocal_QuantityRemaining))
      (elif (.EmptySlotFound (CallFunction|AnyEmptySlotsAvailable))
        (bind _success (CallFunction|CreateNewStack ItemID 1))
        (if _success
          (Math|Integer|DecrementInt (LocalVariables|GetLocal_QuantityRemaining))
          (else
            (LocalVariables|SetLocal_HasFailed true)))
        (else
          (LocalVariables|SetLocal_HasFailed true)))))
  (return (not (LocalVariables|GetLocal_HasFailed)) (LocalVariables|GetLocal_QuantityRemaining)))

(fn RemovefromInventory)

(fn FindSlot
  (params (ItemID :type Name))
  (for (_array_element _array_index) (Variables|Default|GetContent)
    (if (== (.ItemID (Utilities|Struct|BreakInventorySlotStruct _array_element)) ItemID)
      (if (< (.Quantity (Utilities|Struct|BreakInventorySlotStruct _array_element)) (CallFunction|GetMaxStackSize ItemID))
        (return _array_index true))))
  (return -1 false))

(fn GetMaxStackSize
  (params (ItemID :type Name))
  (bind _returnvalue (Utilities|GetDataTableRow "/Game/Equipment/ItemData.ItemData" ItemID)
    (:then
      (return (Utilities|Struct|BreakItemStruct _returnvalue)))
    (:RowNotFound
      (return -1))))

(fn AddtoStack
  (params (Index :type Integer) (Quantity :type Integer))
  (bind _content (Variables|Default|GetContent))
  (bind _output (Utilities|Array|Get(acopy) _content Index))
  (Utilities|Array|SetArrayElem (Variables|Default|GetContent) Index (Utilities|Struct|MakeInventorySlotStruct (.itemid _output) (+ (.quantity _output) Quantity))))

(fn AnyEmptySlotsAvailable
  (for (_array_element _array_index) (Variables|Default|GetContent)
    (if (== 0 (.Quantity (Utilities|Struct|BreakInventorySlotStruct _array_element)))
      (return true _array_index)))
  (return false -1))

(fn CreateNewStack
  (params (ItemID :type Name) (Quantity :type Integer))
  (bind (_emptyslotfound _index) (CallFunction|AnyEmptySlotsAvailable))
  (if _emptyslotfound
    (Utilities|Array|SetArrayElem (Variables|Default|GetContent) _index (Utilities|Struct|MakeInventorySlotStruct ItemID Quantity))
    (return true)
    (else
      (return false))))

(fn DEBUGPrintContents
  (for (_array_element _array_index) (Variables|Default|GetContent)
    (Development|PrintString (Utilities|String|Append (Utilities|String|ToString(Integer) _array_index) ":" (Utilities|String|ToString(Name) (.ItemID (Utilities|Struct|BreakInventorySlotStruct _array_element))) " = " (Utilities|String|ToString(Integer) (.Quantity (Utilities|Struct|BreakInventorySlotStruct _array_element)))))))