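; BP_TestInteraction is a test interactable actor with a cube that responds to focus and interact interface events.
; Focus toggles custom depth rendering on the cube.
; Interact calls InteractOnServer, which flips the InteractToggle boolean, whose RepNotify prints the new value.
; A getter exposes its Widget as the interaction widget reference.
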(event Custom|InteractOnServer
  (Variables|Default|SetInteractToggle (not (Variables|Default|GetInteractToggle))))

(event EventBeginPlay)

(event Collision|EventActorBeginOverlap
  (params (OtherActor :type Actor%20Object%20Reference)))

(event EventTick
  (params (DeltaSeconds :type Float%20%28single-precision%29)))

(event EventInterfaceToggleFocus
  (params (Focus :type Boolean))
  (Rendering|SetRenderCustomDepth (Variables|Default|GetCube) Focus))

(event EventInterfaceInteract
  (CallFunction|InteractonServer))

(fn ConstructionScript)

(fn OnRepInteractToggle
  (Development|PrintText (Utilities|Text|ToText(Boolean) (Variables|Default|GetInteractToggle))))

(fn GetInteractionWidgetRef
  (return (Variables|Default|GetWidget)))