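; Interaction component that finds the interaction area the player is looking at and triggers its interaction.
; Every tick it line-traces from the player camera and toggles focus as the hit actor changes, accepting only Box and CustomShape interact areas.
; TryToInteract passes a focused area with no positive InteractDuration to InteractOnServer, which sends an interface message to the area's parent actor.
; Areas with a positive duration get no handling here.
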(event Custom|TryToInteract
  (params (In :type Boolean))
  (if In
    (if (Variables|Default|GetIsTracingInteractionArea)
      (bind _output_get (Variables|Default|SetInteractDuration (Variables|/Game/Blueprints/BP_InteractArea_Master.BP_InteractArea_Master_C|GetInteractDuration (Variables|Default|GetFocusedInteractionArea))))
      (if (not (> _output_get 0.0))
        (CallFunction|InteractonServer (Variables|Default|GetFocusedInteractionArea))))))

(event Custom|InteractOnServer
  (params (InteractionArea :type BP%20Interact%20Area%20Master%20Object%20Reference))
  (Class|BIInteract|InterfaceInteract(Message) (Actor|GetParentActor InteractionArea)))

(event EventTick
  (params (DeltaSeconds :type Float%20%28single-precision%29))
  (CallFunction|Trace))

(fn Trace
  (bind _returnvalue (Game|GetPlayerCameraManager 0))
  (bind _returnvalue_2 (Transformation|GetActorLocation _returnvalue))
  (bind (_outhit _returnvalue_3) (Collision|LineTraceByChannel _returnvalue_2 (+ _returnvalue_2 (* (Math|Vector|GetForwardVector (Transformation|GetActorRotation _returnvalue)) (Variables|Default|GetLength))) "TraceTypeQuery1" false 0 "None"))
  (if _returnvalue_3
    (if (!= (Variables|Default|GetFocusedActor) (.HitActor (Collision|BreakHitResult _outhit)))
      (Variables|Default|SetFocusedActor (.HitActor (Collision|BreakHitResult _outhit)))
      (CallFunction|TraceInteractionArea (or (== (Utilities|GetClass (.HitActor (Collision|BreakHitResult _outhit))) "/Game/Blueprints/BP_InteractArea_CustomShape.BP_InteractArea_CustomShape_C") (== (Utilities|GetClass (.HitActor (Collision|BreakHitResult _outhit))) "/Game/Blueprints/BP_InteractArea_Box.BP_InteractArea_Box_C"))))
    (else
      (CallFunction|TraceInteractionArea false))))

(fn TraceInteractionArea
  (params (Trace :type Boolean))
  (if Trace
    (if (Variables|Default|GetIsTracingInteractionArea)
      (Default|ToggleFocus (Variables|Default|GetFocusedInteractionArea) false))
    (bind _asbp_interact_area_master (Utilities|Casting|CastToBP_InteractArea_Master (Variables|Default|GetFocusedActor)))
    (bind _output_get (Variables|Default|SetFocusedInteractionArea _asbp_interact_area_master))
    (Default|ToggleFocus _output_get true)
    (Variables|Default|SetIsTracingInteractionArea true)
    (elif (Variables|Default|GetIsTracingInteractionArea)
      (Variables|Default|SetIsTracingInteractionArea false)
      (Default|ToggleFocus (Variables|Default|GetFocusedInteractionArea) false)
      (Variables|Default|SetFocusedActor 0)
      (Variables|Default|SetFocusedInteractionArea 0))))