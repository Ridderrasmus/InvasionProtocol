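; Actor component that lets the player pick up, carry and drop physics objects in front of the camera.
; It adds a Physics Handle to its owner at BeginPlay, and GrabObject line-traces from the camera to grab movable components within a mass limit.
; Each tick it rechecks that limit, then either moves the held object's target to the hold distance along the view or drops it.
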(event Custom|GrabObject
  (bind _returnvalue (Game|GetPlayerCameraManager 0))
  (bind _returnvalue_2 (Transformation|GetActorLocation _returnvalue))
  (bind (_outhit _returnvalue_3) (Collision|LineTraceByChannel _returnvalue_2 (+ _returnvalue_2 (* (Math|Vector|GetForwardVector (Transformation|GetActorRotation _returnvalue)) (Variables|Default|GetDistanceToHeldObject))) "TraceTypeQuery1" false 0 "None"))
  (if _returnvalue_3
    ;[1 1 1] Check whether target actor can be picked up
    (bind _iscarryable (CallFunction|IsTargetActorCarryable (.HitComponent (Collision|BreakHitResult _outhit))))
    (if _iscarryable
      (Physics|Components|PhysicsHandle|GrabComponentatLocationwithRotation (Variables|Default|GetPhysicsHandle) (.HitComponent (Collision|BreakHitResult _outhit)) "None" (Transformation|GetWorldLocation (.HitComponent (Collision|BreakHitResult _outhit))) "0, 0, 0")
      (Variables|Default|SetIsCarryingObject true))))

(event Custom|DropObject
  (if (Variables|Default|GetIsCarryingObject)
    (Physics|Components|PhysicsHandle|ReleaseComponent (Variables|Default|GetPhysicsHandle))
    (Variables|Default|SetIsCarryingObject false)))

(event EventBeginPlay
  (bind _returnvalue (Game|AddComponentbyClass (Components|GetOwner) "/Script/Engine.PhysicsHandleComponent"))
  (Variables|Default|SetPhysicsHandle _returnvalue))

(event EventTick
  (params (DeltaSeconds :type Float%20%28single-precision%29))
  ;[1 1 1] Abort cycle if not carrying an object
  (if (Variables|Default|GetIsCarryingObject)
    ;[1 1 1] Check if actor is carryable in cycle, if yes then update location if not then drop object
    (bind _iscarryable (CallFunction|IsTargetActorCarryable (Class|PhysicsHandleComponent|GetGrabbedComponent (Variables|Default|GetPhysicsHandle))))
    (if _iscarryable
      (CallFunction|UpdateCarriedObjectLocation)
      (else
        (CallFunction|DropObject)))))

(fn IsTargetActorCarryable
  (params (TargetActor :type Primitive%20Component%20Object%20Reference))
  (bind _maxcarryweight (Variables|Default|GetMaxCarryWeight))
  ;[1 1 1] Checks whether defined maxcarryweight is less than or equal to zero OR if the object isn't movable
  (if (or (Utilities|Enum|NotEqual(Enum) (Variables|/Script/Engine.SceneComponent|GetMobility TargetActor) "Movable") (<= _maxcarryweight 0.0))
    (return false)
    (else
      (return (>= _maxcarryweight (Physics|GetMass TargetActor))))))

(fn UpdateCarriedObjectLocation
  (bind _returnvalue (Game|GetPlayerCameraManager 0))
  (Physics|Components|PhysicsHandle|SetTargetLocation (Variables|Default|GetPhysicsHandle) (+ (Transformation|GetActorLocation _returnvalue) (* (Math|Vector|GetForwardVector (Transformation|GetActorRotation _returnvalue)) (Variables|Default|GetDistanceToHeldObject)))))