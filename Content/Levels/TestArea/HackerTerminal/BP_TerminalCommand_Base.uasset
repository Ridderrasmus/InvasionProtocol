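; BP_TerminalCommand_Base is the base class for commands in the hacker terminal.
; It exposes a primary name plus alternative names as one list, and validates input by comparing the parameter count to an expected number, with a formatted error message.
; ExecuteTerminalCommand receives parameters, the terminal and a target device, and by default fails with a "Command not defined!" error.
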(fn ValidateInput
  (params (Parameters :type Array%20of%20Strings))
  (return (== (Utilities|Array|Length Parameters) (Variables|Default|GetExpectedNumberOfParameters)) (Utilities|String|ToString(Text) (Utilities|Text|FormatText "The command {CommandName} takes {NumberOfParameters} parameters." (Variables|Default|GetPrimaryCommandName) (Variables|Default|GetExpectedNumberOfParameters)))))

(fn GetCommandNames
  (Utilities|Array|Add (LocalVariables|GetAllCommands) (Variables|Default|GetPrimaryCommandName))
  (Utilities|Array|AppendArray (LocalVariables|GetAllCommands) (Variables|Default|GetAlternativeCommandNames))
  (return (LocalVariables|GetAllCommands)))

(fn ExecuteTerminalCommand
  (params (Parameters :type Array%20of%20Strings) (HackerTerminal :type AC%20Hacker%20Terminal%20Object%20Reference) (TargetDevice :type AC%20Hackable%20Object%20Reference))
  (return false "Command not defined!"))