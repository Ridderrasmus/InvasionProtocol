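; Actor component for a hacker terminal that turns typed command strings into actions on the currently connected hackable device.
; On BeginPlay it instantiates the connect, text hack and light hack command objects, mapping each of their names to the instance.
; Input is parsed, looked up and parameter-checked before the command object executes, with failures printed in red.
; It also keeps a name-keyed registry of hackable devices for lookup.
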(event Custom|HandleTerminalCommand
  (params (TerminalCommandString :type String))
  ;[1 1 1] Validate the entered string is a valid command
  (bind (_isvalid _command _commandparameters _errormessage) (CallFunction|ValidateTerminalCommand TerminalCommandString))
  (if _isvalid
    ;[1 1 1] Validate that the command has correct number of parameters
    (bind (_isvalid_2 _errormessage_2) (Default|ValidateInput _command _commandparameters))
    (if _isvalid_2
      (bind (_success _errormessage_3) (Default|ExecuteTerminalCommand _command _commandparameters self (Variables|Default|GetCurrentConnectedDevice)))
      (if (not _success)
        (Development|PrintString _errormessage_3 true true "(R=1.000000,G=0.000000,B=0.007289,A=1.000000)" 1e+01))
      (else
        (Development|PrintString _errormessage_2 true true "(R=1.000000,G=0.000000,B=0.007289,A=1.000000)" 1e+01)))
    (else
      (Development|PrintString _errormessage true true "(R=1.000000,G=0.000000,B=0.007289,A=1.000000)" 1e+01))))

(event EventBeginPlay
  ;[1 1 1] Todo - better...
  (CallFunction|InitializeTerminalCommands))

(fn ValidateTerminalCommand
  (params (TerminalString :type String))
  (bind _output_get (LocalVariables|SetCurrentCommand (Utilities|String|ParseIntoArray TerminalString " ")))
  (if (.ReturnValue (Utilities|Map|Find (Variables|Default|GetTerminalCommands) (Utilities|Array|Get(acopy) _output_get)))
    (LocalVariables|SetTerminalCommandFound (.Value (Utilities|Map|Find (Variables|Default|GetTerminalCommands) (Utilities|Array|Get(acopy) _output_get))))
    (Utilities|Array|RemoveIndex (LocalVariables|GetCurrentCommand))
    (return true (LocalVariables|GetTerminalCommandFound) (LocalVariables|GetCurrentCommand) "")
    (else
      (return false 0 0 (Utilities|String|Append (Utilities|Array|Get(acopy) _output_get) (Utilities|String|ToString(Text) (LocalVariables|GetInvalidCommandText)))))))

(fn AddHackableDevice
  (params (DeviceToAdd :type AC%20Hackable%20Object%20Reference))
  (Utilities|Map|Add (Variables|Default|GetAllHackableDevices) (Variables|/Game/Levels/TestArea/AC_Hackable.AC_Hackable_C|GetDeviceName DeviceToAdd) DeviceToAdd))

(fn InitializeTerminalCommands
  (CallFunction|AddTerminalCommand "/Game/Levels/TestArea/HackerTerminal/BP_TerminalCommandConnect_Child.BP_TerminalCommandConnect_Child_C")
  (CallFunction|AddTerminalCommand "/Game/Levels/TestArea/HackerTerminal/BP_TerminalCommandTextHack_Child.BP_TerminalCommandTextHack_Child_C")
  (CallFunction|AddTerminalCommand "/Game/Levels/TestArea/HackerTerminal/BP_TerminalCommandLightHack_Child.BP_TerminalCommandLightHack_Child_C"))

(fn AddTerminalCommand
  (params (TerminalCommand :type BP%20Terminal%20Command%20Base%20Class%20Reference))
  (bind _returnvalue (Game|ConstructObjectfromClass TerminalCommand))
  (bind _commands (Default|GetCommandNames _returnvalue))
  (bind _output_get (LocalVariables|SetCommandNames _commands))
  (for _array_element _output_get
    (Utilities|Map|Add (Variables|Default|GetTerminalCommands) _array_element _returnvalue)))

(fn GetDevicebyName
  (params (DeviceName :type String))
  (bind _allhackabledevices (Variables|Default|GetAllHackableDevices))
  (bind (_value _returnvalue) (Utilities|Map|Find _allhackabledevices DeviceName))
  (return _value _returnvalue))