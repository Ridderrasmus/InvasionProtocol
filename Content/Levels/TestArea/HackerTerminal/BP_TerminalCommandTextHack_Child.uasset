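; Terminal command Blueprint for the hacker terminal that starts string-based hacks on a target device.
; ExecuteTerminalCommand stores the target device, finds all of its hacks matching HackType, and passes the first command parameter to each through BeginHackString.
; It reports success whenever the device is valid, even if no hacks match, and returns an error when the device is null.
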(fn ExecuteTerminalCommand
  (params (Parameters :type Array%20of%20Strings) (HackerTerminal :type AC%20Hacker%20Terminal%20Object%20Reference) (TargetDevice :type AC%20Hackable%20Object%20Reference))
  (bind _output_get (LocalVariables|SetTarget%20Device TargetDevice))
  (if (Utilities|IsValid _output_get)
    (bind _matchinghacks (Default|FindHacksbyType (LocalVariables|GetTarget%20Device) (Variables|Default|GetHackType)))
    (for _array_element _matchinghacks
      (Default|BeginHackString _array_element (Utilities|Array|Get(acopy) Parameters)))
    (return true "")
    (else
      (return false "Device is null!"))))