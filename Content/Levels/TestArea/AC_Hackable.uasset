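; AC_Hackable is an actor component that makes its owner a hackable device for the player's hacker terminal.
; On BeginPlay it gathers the owner's BI_Hack components that cast to AC_HackBase and groups them by HackType in a map of array-wrapping structs.
; It then registers itself with the first AC_HackerTerminal on player pawn 0.
; FindHacksByType returns the stored hacks for a requested type.
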(event EventBeginPlay
  ;[1 1 1] Setup
  (CallFunction|GetHackReferences)
  (CallFunction|RegisterDeviceatHacker))

(fn GetHackReferences
  (for _array_element (Class|Actor|GetComponentsbyInterface (Components|GetOwner) "/Game/Levels/TestArea/BI_Hack.BI_Hack_C")
    (bind _asac_hack_base (Utilities|Casting|CastToAC_HackBase _array_element))
    (if (.ReturnValue (Utilities|Map|Find (Variables|Default|GetAvailableHacks) (Variables|/Game/Levels/TestArea/AC_HackBase.AC_HackBase_C|GetHackType _asac_hack_base)))
      (Utilities|Array|Add (Utilities|Struct|BreakS_AvailableHacksOfType (.Value (Utilities|Map|Find (Variables|Default|GetAvailableHacks) (Variables|/Game/Levels/TestArea/AC_HackBase.AC_HackBase_C|GetHackType _asac_hack_base)))) _asac_hack_base)
      (else
        (Utilities|Map|Add (Variables|Default|GetAvailableHacks) (Variables|/Game/Levels/TestArea/AC_HackBase.AC_HackBase_C|GetHackType _asac_hack_base) (Utilities|Struct|MakeS_AvailableHacksOfType (Utilities|Array|MakeArray _asac_hack_base)))))))

(fn RegisterDeviceatHacker
  ;[1 1 1] Register the device with the hacker
  (bind _array_element (Utilities|Array|ForEachLoopwithBreak (Actor|GetComponentsByClass (Game|Player|GetPlayerPawn 0) "/Game/Levels/TestArea/HackerTerminal/AC_HackerTerminal.AC_HackerTerminal_C") :!label _label)
    (:LoopBody
      (Default|AddHackableDevice _array_element self)
      (goto _label Break))))

(fn FindHacksbyType
  (params (HackType :type HackType%20Enum :default "NewEnumerator6"))
  (bind _availablehacks (Variables|Default|GetAvailableHacks))
  (bind (_value _returnvalue) (Utilities|Map|Find _availablehacks HackType))
  (if _returnvalue
    (return (Utilities|Struct|BreakS_AvailableHacksOfType _value))
    (else
      (return 0))))